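; Elevator actor that the player toggles between its start position and a configurable target location with the Interact input.
; A box trigger opens a gate when the ThirdPersonCharacter overlaps and closes it on exit, so input only works inside the box.
; Interact checks an IsUp flag to play or reverse a timeline that lerps the plane's relative location to or from ElevatorLocation.
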(event `self.ReceiveBeginPlay`
  ;[1 1 1] Cast to player
  (`self.EnableInput` (`GameplayStatics.GetPlayerController` 0)))

(event `ElevatorMove`
  ;[1 1 1] Movement Function
  (set `self.IsUp` true)
  (bind (_direction _alpha) (`Timeline|ElevatorMovment` :!label _label)
    (:`Update`
      (`SceneComponent.K2_SetRelativeLocationAndRotation` :`self` (`self.Plane`) :`NewLocation` (`KismetMathLibrary.VLerp` (0.0 0.0 0.0) (`self.ElevatorLocation`) _alpha)))))

(event `Elevator Reverse`
  ;[1 1 1] Movement Function
  (set `self.IsUp` false)
  (goto _label :!via `Reverse`))

(event `InputAction|Interact` :consume false
  (params (Key :type "Key Structure"))
  ;[1 1 1] Interaction function
  (:`Pressed`
    (`/Engine/EditorBlueprintResources/StandardMacros.Gate` true :!label _label_2
      (:`Exit`
        (if (`self.IsUp`)
          (`self.Elevator Reverse`)
          (else
            (`self.ElevatorMove`)))))))

(event `self.Box.OnComponentBeginOverlap`
  (params (OverlappedComponent :type "PrimitiveComponent Object Reference") (OtherActor :type "Actor Object Reference") (OtherComp :type "PrimitiveComponent Object Reference") (OtherBodyIndex :type Integer) (bFromSweep :type Boolean) (SweepResult :type "HitResult Structure (by ref)"))
  ;[1 1 1] Interaction function
  (cast `/Game/ThirdPersonBP/Blueprints/ThirdPersonCharacter` OtherActor)
  (goto _label_2 :!via `Open`))

(event `self.Box.OnComponentEndOverlap`
  (params (OverlappedComponent :type "PrimitiveComponent Object Reference") (OtherActor :type "Actor Object Reference") (OtherComp :type "PrimitiveComponent Object Reference") (OtherBodyIndex :type Integer))
  ;[1 1 1] Interaction function
  (cast `/Game/ThirdPersonBP/Blueprints/ThirdPersonCharacter` OtherActor)
  (goto _label_2 :!via `Close`))

(fn `UserConstructionScript`)