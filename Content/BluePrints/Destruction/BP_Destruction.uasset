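; BP_Destruction is a destructible chest prop with a color-changing point light.
; A looping timer started on BeginPlay periodically gives the light a random color.
; Fracturing the destructible mesh plays an explosion sound at a location.
; The box overlap only casts to ThirdPersonCharacter, as the radius damage node meant to break the chest is left unconnected.
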(event `self.Box.OnComponentBeginOverlap`
  (params (OverlappedComponent :type "PrimitiveComponent Object Reference") (OtherActor :type "Actor Object Reference") (OtherComp :type "PrimitiveComponent Object Reference") (OtherBodyIndex :type Integer) (bFromSweep :type Boolean) (SweepResult :type "HitResult Structure (by ref)"))
  ;[1 1 1] Destructable funcion
  (cast `/Game/ThirdPersonBP/Blueprints/ThirdPersonCharacter` OtherActor))

(event `Light timer`
  ;[1 1 1] Lighting function
  (`LightComponent.SetLightColor` (`self.PointLight`) (make `LinearColor` (`KismetMathLibrary.RandomFloatInRange` 0.0 1.0) (`KismetMathLibrary.RandomFloatInRange` 0.0 1.0) (`KismetMathLibrary.RandomFloatInRange` 0.0 1.0) 1.0) true))

(event `self.ReceiveBeginPlay`
  ;[1 1 1] Lighting function
  (`KismetSystemLibrary.K2_SetTimer` null "Light timer" 2.0 true))

(event `self.MESH_Chest_DM.OnComponentFracture`
  (params (HitPoint :type "Vector Structure (by ref)") (HitDirection :type "Vector Structure (by ref)"))
  ;[1 1 1] Sound Effect for Box Fracture
  (`GameplayStatics.PlaySoundAtLocation` "/Game/StarterContent/Audio/Explosion_Cue.Explosion_Cue"))

(fn `UserConstructionScript`)