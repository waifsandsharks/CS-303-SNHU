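; Hover component that makes its owning actor float above surfaces using physics forces.
; On BeginPlay it caches the owner's first primitive component and enables physics simulation on it.
; Each tick it traces downward and, on a hit, pushes that body along the surface normal with force fading linearly over the trace length.
; Hits also apply linear and angular damping, which is never reset when the trace misses.
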(event `self.ReceiveBeginPlay`
  (bind _output_get (set `self.Primitive Component` (`|GetArrayItem` (`Actor.K2_GetComponentsByClass` (`self.GetOwner`) "/Script/Engine.PrimitiveComponent"))))
  (`PrimitiveComponent.SetSimulatePhysics` _output_get true))

(event `self.ReceiveTick`
  (params (DeltaSeconds :type "Float (single-precision)"))
  (bind _returnvalue (`self.K2_GetComponentLocation`))
  (bind (_outhit _returnvalue_2) (`KismetSystemLibrary.LineTraceSingle` _returnvalue (- _returnvalue (`KismetMathLibrary.MakeVector` 0.0 0.0 (`self.Trace Length`))) "TraceTypeQuery1"))
  (if _returnvalue_2
    (bind (_bblockinghit _binitialoverlap _time _distance _location _impactpoint _normal _impactnormal) (`GameplayStatics.BreakHitResult` _outhit))
    (`PrimitiveComponent.AddForce` (`self.Primitive Component`) (* _impactnormal (`KismetMathLibrary.Lerp` 500000.0 0.0 (/ (`KismetMathLibrary.VSize` (- _location (`self.K2_GetComponentLocation`))) (`self.Trace Length`)))) "None" false)
    (`PrimitiveComponent.SetLinearDamping` (`self.Primitive Component`) (`self.Linear Damping`))
    (`PrimitiveComponent.SetAngularDamping` (`self.Primitive Component`) (`self.Angular Damping`))))