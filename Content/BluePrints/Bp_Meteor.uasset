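; Meteor actor that moves along a path of six control points through an InterpToMovement component.
; The Construction Script builds the control points from six location variables, all relative to the actor, and applies the Duration variable as the travel time.
; The component drives all motion, as the event graph holds only an empty BeginPlay.
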(event `self.ReceiveBeginPlay`)

(fn `UserConstructionScript`
  (bind _interptomovement (`self.InterpToMovement`))
  (set `InterpToMovementComponent.ControlPoints` (`|MakeArray` (make `InterpControlPoint` (`self.Location1`)) (make `InterpControlPoint` (`self.Location2`)) (make `InterpControlPoint` (`self.Location3`)) (make `InterpControlPoint` (`self.Location4`)) (make `InterpControlPoint` (`self.Location5`)) (make `InterpControlPoint` (`self.Location6`))) _interptomovement)
  (set `InterpToMovementComponent.Duration` (`self.Duration`) _interptomovement))